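; Player character for a top-down flipbook game, with movement, directional melee and dodge, damage and death handling.
; Tick and Attack share a chain that picks flipbooks by player number, facing and state, damages directional hitbox overlaps, expires old inputs and updates HUD values.
; Music keys fill a timestamped three-key buffer that CheckCombos matches against WomboCombo to trigger fireball, haste or a heal spawn.
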(event Custom|HitchangeEvent
  (Utilities|FlowControl|Delay 0.2)
  (Sprite|SetSpriteColor (Variables|Default|GetSprite) "(R=1.000000,G=1.000000,B=1.000000,A=1.000000)"))

(event EventBeginPlay
  (bind _returnvalue (Game|GetCurrentLevelName true))
  (if (Utilities|Enum|Equal(Enum) _returnvalue "Level01")
    (bind _returnvalue_2 (UserInterface|CreateWidget "/Game/blueprints/HealthBars.HealthBars_C"))
    (bind _output_get (Variables|Default|SetHUD%20Reference _returnvalue_2))
    (UserInterface|Viewport|AddtoViewport _output_get 0)))

(event Collision|EventActorBeginOverlap
  (params (OtherActor :type Actor%20Object%20Reference)))

(event EventTick
  (params (DeltaSeconds :type Float%20%28single-precision%29))
  (bind _inputstiming (Variables|Default|GetInputsTiming))
  ;[1 1 1] Animates Player
  (Pawn|Character|SetAnimation)
  ;[1 1 1] sets delay so attack anim can play, think hitbox problem is either in here or because we don't want it to be on begin overlap, not sure.
  (if (Variables|Default|GetisAttacking)
    (CallFunction|StartSwing)
    (Utilities|FlowControl|Delay 0.4)
    (Variables|Default|SetisAttacking false)
    (CallFunction|EndSwing))
  ;[1 1 1] removes keys from the buffer if they stay in there too long
  (if (> (Utilities|Array|Length _inputstiming) 0)
    (if (< (Utilities|Array|Get(acopy) _inputstiming) (- (Math|DateTime|Now) (Math|Timespan|MakeTimespan 0 0 0 5)))
      (Utilities|Array|RemoveIndex _inputstiming)
      (Utilities|Array|RemoveIndex (Variables|Default|GetInputs))))
  (CallFunction|UpdateHud))

(event Input|ActionEvents|InputActionAttack
  (params (Key :type Key%20Structure :default "AnyKey"))
  (bind _inputstiming (Variables|Default|GetInputsTiming))
  ;[1 1 1] Animates Attack
  (:Pressed
    (Variables|Default|SetisAttacking true)
    ;[1 1 1] Animates Player
    (Pawn|Character|SetAnimation)
    ;[1 1 1] sets delay so attack anim can play, think hitbox problem is either in here or because we don't want it to be on begin overlap, not sure.
    (if (Variables|Default|GetisAttacking)
      (CallFunction|StartSwing)
      (Utilities|FlowControl|Delay 0.4)
      (Variables|Default|SetisAttacking false)
      (CallFunction|EndSwing))
    ;[1 1 1] removes keys from the buffer if they stay in there too long
    (if (> (Utilities|Array|Length _inputstiming) 0)
      (if (< (Utilities|Array|Get(acopy) _inputstiming) (- (Math|DateTime|Now) (Math|Timespan|MakeTimespan 0 0 0 5)))
        (Utilities|Array|RemoveIndex _inputstiming)
        (Utilities|Array|RemoveIndex (Variables|Default|GetInputs))))
    (CallFunction|UpdateHud)))

(event Input|ActionEvents|InputActionQuit
  (params (Key :type Key%20Structure :default "AnyKey"))
  (:Released
    (Game|QuitGame 0 "Quit")))

(event Input|ActionEvents|InputActionMusicUp
  (params (Key :type Key%20Structure :default "AnyKey"))
  (bind _returnvalue (Transformation|GetActorLocation))
  (bind _charactermovement (Variables|Character|GetCharacterMovement))
  (bind _sprite (Variables|Default|GetSprite))
  (:Pressed
    (CallFunction|AddInput "I")
    (bind _didspecial (Pawn|Character|CheckCombos))
    (Variables|Default|SetdidSpecial false)
    (if _didspecial
      (switch Utilities|FlowControl|Switch|SwitchonComboEnum (Variables|Default|GetLastCombo)
        (:NewEnumerator5
          (if (Variables|Default|GetcanFireball)
            (Development|PrintString "FIREBALL")
            (Game|SpawnActorfromClass "/Game/blueprints/playerFire.playerFire_C" (Math|Transform|MakeTransform (Transformation|GetActorLocation self) "0, 0,0.000000") "Undefined" 0 self)))
        (:NewEnumerator6
          (Development|PrintString "HASTE")
          (Variables|Default|SetHP (+ (Variables|Default|GetHP) 0))
          (Sprite|SetSpriteColor _sprite "(R=0.537255,G=0.607843,B=0.015686,A=1.000000)")
          (Variables|/Script/Engine.CharacterMovementComponent|SetMaxWalkSpeed _charactermovement 6e+02)
          (Utilities|FlowControl|Delay 5.0)
          (Variables|/Script/Engine.CharacterMovementComponent|SetMaxWalkSpeed _charactermovement 4e+02)
          (Sprite|SetSpriteColor _sprite "(R=1.000000,G=1.000000,B=1.000000,A=1.000000)"))
        (:NewEnumerator7
          (Development|PrintString "EMPOWER")
          (switch Utilities|FlowControl|Switch|SwitchonMovement (Variables|Default|GetLastMovement)
            (:NewEnumerator0
              (Variables|Default|SethealSpawn (+ _returnvalue "0,-30.000000,0.000000")))
            (:NewEnumerator1
              (Variables|Default|SethealSpawn (+ _returnvalue "0,30.000000, 0")))
            (:NewEnumerator2
              (Variables|Default|SethealSpawn (+ _returnvalue "-30.000000, 0, 0")))
            (:NewEnumerator3
              (Variables|Default|SethealSpawn (+ _returnvalue "30.000000, 0, 0"))))
          (Game|SpawnActorfromClass "/Game/blueprints/playerHeal.playerHeal_C" (Math|Transform|MakeTransform (Variables|Default|GethealSpawn) "0, 0,0.000000") "Undefined" 0 self))))))

(event Input|ActionEvents|InputActionMusicLeft
  (params (Key :type Key%20Structure :default "AnyKey"))
  (bind _returnvalue (Transformation|GetActorLocation))
  (bind _charactermovement (Variables|Character|GetCharacterMovement))
  (bind _sprite (Variables|Default|GetSprite))
  (:Pressed
    (CallFunction|AddInput "J")
    (bind _didspecial (Pawn|Character|CheckCombos))
    (Variables|Default|SetdidSpecial false)
    (if _didspecial
      (switch Utilities|FlowControl|Switch|SwitchonComboEnum (Variables|Default|GetLastCombo)
        (:NewEnumerator5
          (if (Variables|Default|GetcanFireball)
            (Development|PrintString "FIREBALL")
            (Game|SpawnActorfromClass "/Game/blueprints/playerFire.playerFire_C" (Math|Transform|MakeTransform (Transformation|GetActorLocation self) "0, 0,0.000000") "Undefined" 0 self)))
        (:NewEnumerator6
          (Development|PrintString "HASTE")
          (Variables|Default|SetHP (+ (Variables|Default|GetHP) 0))
          (Sprite|SetSpriteColor _sprite "(R=0.537255,G=0.607843,B=0.015686,A=1.000000)")
          (Variables|/Script/Engine.CharacterMovementComponent|SetMaxWalkSpeed _charactermovement 6e+02)
          (Utilities|FlowControl|Delay 5.0)
          (Variables|/Script/Engine.CharacterMovementComponent|SetMaxWalkSpeed _charactermovement 4e+02)
          (Sprite|SetSpriteColor _sprite "(R=1.000000,G=1.000000,B=1.000000,A=1.000000)"))
        (:NewEnumerator7
          (Development|PrintString "EMPOWER")
          (switch Utilities|FlowControl|Switch|SwitchonMovement (Variables|Default|GetLastMovement)
            (:NewEnumerator0
              (Variables|Default|SethealSpawn (+ _returnvalue "0,-30.000000,0.000000")))
            (:NewEnumerator1
              (Variables|Default|SethealSpawn (+ _returnvalue "0,30.000000, 0")))
            (:NewEnumerator2
              (Variables|Default|SethealSpawn (+ _returnvalue "-30.000000, 0, 0")))
            (:NewEnumerator3
              (Variables|Default|SethealSpawn (+ _returnvalue "30.000000, 0, 0"))))
          (Game|SpawnActorfromClass "/Game/blueprints/playerHeal.playerHeal_C" (Math|Transform|MakeTransform (Variables|Default|GethealSpawn) "0, 0,0.000000") "Undefined" 0 self))))))

(event Input|ActionEvents|InputActionMusicRight
  (params (Key :type Key%20Structure :default "AnyKey"))
  (bind _returnvalue (Transformation|GetActorLocation))
  (bind _charactermovement (Variables|Character|GetCharacterMovement))
  (bind _sprite (Variables|Default|GetSprite))
  (:Pressed
    (CallFunction|AddInput "L")
    (bind _didspecial (Pawn|Character|CheckCombos))
    (Variables|Default|SetdidSpecial false)
    (if _didspecial
      (switch Utilities|FlowControl|Switch|SwitchonComboEnum (Variables|Default|GetLastCombo)
        (:NewEnumerator5
          (if (Variables|Default|GetcanFireball)
            (Development|PrintString "FIREBALL")
            (Game|SpawnActorfromClass "/Game/blueprints/playerFire.playerFire_C" (Math|Transform|MakeTransform (Transformation|GetActorLocation self) "0, 0,0.000000") "Undefined" 0 self)))
        (:NewEnumerator6
          (Development|PrintString "HASTE")
          (Variables|Default|SetHP (+ (Variables|Default|GetHP) 0))
          (Sprite|SetSpriteColor _sprite "(R=0.537255,G=0.607843,B=0.015686,A=1.000000)")
          (Variables|/Script/Engine.CharacterMovementComponent|SetMaxWalkSpeed _charactermovement 6e+02)
          (Utilities|FlowControl|Delay 5.0)
          (Variables|/Script/Engine.CharacterMovementComponent|SetMaxWalkSpeed _charactermovement 4e+02)
          (Sprite|SetSpriteColor _sprite "(R=1.000000,G=1.000000,B=1.000000,A=1.000000)"))
        (:NewEnumerator7
          (Development|PrintString "EMPOWER")
          (switch Utilities|FlowControl|Switch|SwitchonMovement (Variables|Default|GetLastMovement)
            (:NewEnumerator0
              (Variables|Default|SethealSpawn (+ _returnvalue "0,-30.000000,0.000000")))
            (:NewEnumerator1
              (Variables|Default|SethealSpawn (+ _returnvalue "0,30.000000, 0")))
            (:NewEnumerator2
              (Variables|Default|SethealSpawn (+ _returnvalue "-30.000000, 0, 0")))
            (:NewEnumerator3
              (Variables|Default|SethealSpawn (+ _returnvalue "30.000000, 0, 0"))))
          (Game|SpawnActorfromClass "/Game/blueprints/playerHeal.playerHeal_C" (Math|Transform|MakeTransform (Variables|Default|GethealSpawn) "0, 0,0.000000") "Undefined" 0 self))))))

(event Input|ActionEvents|InputActionDodge
  (params (Key :type Key%20Structure :default "AnyKey"))
  (bind _charactermovement (Variables|Character|GetCharacterMovement))
  (:Pressed
    (Development|PrintString "DODGE")
    (switch Utilities|FlowControl|Switch|SwitchonMovement (Variables|Default|GetLastMovement)
      (:NewEnumerator0
        (Physics|AddImpulse _charactermovement "0.000000,-180000.000000, 0" false))
      (:NewEnumerator1
        (Physics|AddImpulse _charactermovement "0.000000,180000.000000, 0" false))
      (:NewEnumerator2
        (Physics|AddImpulse _charactermovement "-180000.000000, 0, 0" false))
      (:NewEnumerator3
        (Physics|AddImpulse _charactermovement "180000.000000, 0, 0" false)))))

(event Input|AxisEvents|InputAxisMovePlayerV
  (params (AxisValue :type Float%20%28single-precision%29))
  ;[1 1 1] Moves the player
  (Pawn|Input|AddMovementInput "0.000000,1.000000, 0" AxisValue false))

(event Input|AxisEvents|InputAxisMovePlayerH
  (params (AxisValue :type Float%20%28single-precision%29))
  ;[1 1 1] Moves the player
  (Pawn|Input|AddMovementInput "1.000000,0.000000,0.000000" AxisValue false))

(fn ConstructionScript)

(fn SetAnimation
  ;[1 1 1] will set the flipboook to dead if hp <=0, don't have death anim so sets to floor
  (if (Variables|Default|GetisDead)
    _
    (else
      _))
  (if (or (!= (Input|AxisValues|GetMovePlayerV) 0.0) (!= (Input|AxisValues|GetMovePlayerH) 0.0))
    (if (Variables|Default|GetisAttacking)
      _
      (else
        (Variables|Default|SetLastMovement (select (> (Input|AxisValues|GetMovePlayerV) 0.0) "NewEnumerator1" (select (< (Input|AxisValues|GetMovePlayerV) 0.0) "NewEnumerator0" (select (> (Input|AxisValues|GetMovePlayerH) 0.0) "NewEnumerator3" "NewEnumerator2")))))))
  (Sprite|SetFlipbook (Variables|Default|GetSprite) (select (Variables|Default|GetisAttacking) (Utilities|Select :Index (Variables|Default|GetplayerNumber) :Option%200 (Utilities|Select :Index (Variables|Default|GetLastMovement) :NewEnumerator0 "/Game/FlipBooks/playerAttackUpLarge.playerAttackUpLarge" :NewEnumerator1 "/Game/FlipBooks/playerAttackDownLarge.playerAttackDownLarge" :NewEnumerator2 "/Game/FlipBooks/playerAttackLeftLarge.playerAttackLeftLarge" :NewEnumerator3 "/Game/FlipBooks/playerAttackRightLarge.playerAttackRightLarge") :Option%201 (Utilities|Select :Index (Variables|Default|GetLastMovement) :NewEnumerator0 "/Game/FlipBooks/player2AttackUpLarge.player2AttackUpLarge" :NewEnumerator1 "/Game/FlipBooks/player2AttackDownLarge.player2AttackDownLarge" :NewEnumerator2 "/Game/FlipBooks/player2AttackLeftLarge.player2AttackLeftLarge" :NewEnumerator3 "/Game/FlipBooks/player2AttackRightLarge.player2AttackRightLarge")) (select (> (Math|Vector|VectorLength (Transformation|GetVelocity)) 0.0) (Utilities|Select :Index (Variables|Default|GetplayerNumber) :Option%200 (Utilities|Select :Index (Variables|Default|GetLastMovement) :NewEnumerator0 "/Game/FlipBooks/walkUp.walkUp" :NewEnumerator1 "/Game/FlipBooks/walkDown.walkDown" :NewEnumerator2 "/Game/FlipBooks/walkLeft.walkLeft" :NewEnumerator3 "/Game/FlipBooks/walkRight.walkRight") :Option%201 (Utilities|Select :Index (Variables|Default|GetLastMovement) :NewEnumerator0 "/Game/FlipBooks/player2WalkUp.player2WalkUp" :NewEnumerator1 "/Game/FlipBooks/player2WalkDown.player2WalkDown" :NewEnumerator2 "/Game/FlipBooks/player2WalkLeft.player2WalkLeft" :NewEnumerator3 "/Game/FlipBooks/player2WalkRight.player2WalkRight")) (Utilities|Select :Index (Variables|Default|GetplayerNumber) :Option%200 (Utilities|Select :Index (Variables|Default|GetLastMovement) :NewEnumerator0 "/Game/FlipBooks/standUp.standUp" :NewEnumerator1 "/Game/FlipBooks/standDown.standDown" :NewEnumerator2 "/Game/FlipBooks/standLeft.standLeft" :NewEnumerator3 "/Game/FlipBooks/standRight.standRight") :Option%201 (Utilities|Select :Index (Variables|Default|GetLastMovement) :NewEnumerator0 "/Game/FlipBooks/player2StandUp.player2StandUp" :NewEnumerator1 "/Game/FlipBooks/player2StandDown.player2StandDown" :NewEnumerator2 "/Game/FlipBooks/player2StandLeft.player2StandLeft" :NewEnumerator3 "/Game/FlipBooks/player2StandRight.player2StandRight"))))))

(fn AddInput
  (params (button :type Key%20Structure :default "AnyKey"))
  (bind _inputstiming (Variables|Default|GetInputsTiming))
  (bind _inputs (Variables|Default|GetInputs))
  (if (>= (Utilities|Array|Length _inputs) 3)
    (Utilities|Array|RemoveIndex _inputs)
    (Utilities|Array|RemoveIndex _inputstiming))
  (Utilities|Array|Add _inputs button)
  (Utilities|Array|Add _inputstiming (Math|DateTime|Now)))

(fn LoseHP
  (params (damage :type Integer))
  (Variables|Default|SetHP (- (Variables|Default|GetHP) damage))
  (Math|Integer|CompareInt (Variables|Default|GetHP) 0
    (:>
      (Sprite|SetSpriteColor (Variables|Default|GetSprite) "(R=1.000000,G=0.000000,B=0.018821,A=1.000000)")
      (CallFunction|HitchangeEvent))
    (:==
      (Variables|Default|SetisDead true :!label _label)
      (Development|PrintString "you died")
      (bind _asinstance_blueprint (Utilities|Casting|CastToinstanceBlueprint (Game|GetGameInstance)))
      (if (Variables|/Game/blueprints/instanceBlueprint.instanceBlueprint_C|GetgodMode _asinstance_blueprint)
        (Development|PrintString "god mode is nice")
        (else
          (bind _returnvalue (UserInterface|CreateWidget "/Game/Blueprints/youDied.youDied_C" (Game|GetPlayerController 0)))
          (UserInterface|Viewport|AddtoViewport _returnvalue 0)
          (Game|OpenLevel(byName) "Level01"))))
    (:<
      (goto _label))))

(fn MusicSpecial
  (params (ComboArray :type Array%20of%20Key%20Structures))
  (for (_array_element _array_index) (Variables|Default|GetInputs)
    (if (== _array_element (Utilities|Array|Get(acopy) ComboArray))
      (Variables|Default|SetdoSpecial false)
      (bind (_array_element_2 _array_index_2) (Utilities|Array|ForEachLoopwithBreak ComboArray)
        (:LoopBody
          (if (== _array_element_2 (Utilities|Array|Get(acopy) (Variables|Default|GetInputs) (+ _array_index_2 _array_index)))
            (Variables|Default|SetdoSpecial true)
            (else
              (Variables|Default|SetdoSpecial false)
              (return false))))
        (:Completed
          (if (Variables|Default|GetdoSpecial)
            (Variables|Default|SetdoSpecial false)
            (Utilities|Array|Clear (Variables|Default|GetInputs))
            (Utilities|Array|Clear (Variables|Default|GetInputsTiming))
            (return true)
            (else
              (return false)))))))
  (if (Variables|Default|GetdoSpecial)
    (Variables|Default|SetdoSpecial false)
    (Utilities|Array|Clear (Variables|Default|GetInputs))
    (Utilities|Array|Clear (Variables|Default|GetInputsTiming))
    (return true)
    (else
      (return false))))

(fn CheckCombos
  (for (_array_element _array_index) (Variables|Default|GetwomboCombo)
    (bind _didspecial (Pawn|Character|MusicSpecial (Utilities|Struct|BreakCombo _array_element)))
    (if _didspecial
      (Development|PrintString (Utilities|String|ToString(Integer) _array_index))
      (switch int _array_index
        (:0
          (Variables|Default|SetLastCombo "NewEnumerator5"))
        (:1
          (Variables|Default|SetLastCombo "NewEnumerator6"))
        (:2
          (Variables|Default|SetLastCombo "NewEnumerator7")))
      (Variables|Default|SetdidSpecial true)))
  (return (Variables|Default|GetdidSpecial)))

(fn UpdateHud
  (bind _inputs (Variables|Default|GetInputs))
  (Variables|Default|SetHP%20Float (/ (Math|Conversions|ToFloat(Integer) (Variables|Default|GetHP)) 3e+01))
  (Variables|Default|SetstrInputs "")
  (for _index (range 0 (- (Utilities|Array|Length _inputs) 1))
    (Variables|Default|SetstrInputs (Utilities|String|Append (Variables|Default|GetstrInputs) (Utilities|String|ToString(Text) (Class|KismetInputLibrary|KeyGetDisplayName (Utilities|Array|Get(acopy) _inputs _index)))))))

(fn TimedRemovefromBuffer)

(fn DamageEnemy
  (params (NewParam :type Actor%20Object%20Reference))
  (bind _returnvalue (Utilities|GetClass NewParam))
  (if (== _returnvalue "/Game/blueprints/zombie.zombie_C")
    (Actor|DestroyActor NewParam)
    (elif (== _returnvalue "/Game/blueprints/chargeEnemy.chargeEnemy_C")
      (bind _ascharge_enemy (Utilities|Casting|CastTochargeEnemy NewParam))
      (switch Utilities|FlowControl|Switch|SwitchonChargeEnum (Variables|/Game/blueprints/chargeEnemy.chargeEnemy_C|GetchargeEnum _ascharge_enemy)
        (:NewEnumerator0
          (Development|PrintString "hit but wasn't tired" :!label _label))
        (:NewEnumerator1
          (goto _label))
        (:NewEnumerator2
          (Default|Die _ascharge_enemy)))
      (elif (== _returnvalue "/Game/blueprints/boss.boss_C")
        (bind _asboss (Utilities|Casting|CastToboss NewParam))
        ;[1 1 1] needs a time delay, isn't working for reasons unknown
        (if (not (Variables|Default|GetBossHit))
          (Default|BossLoseHP _asboss (Variables|Default|GetswingDamage))
          (Variables|Default|SetBossHit true))
        (elif (== _returnvalue "/Game/blueprints/wallPiece.wallPiece_C")
          (Actor|DestroyActor NewParam))))))

(fn StartSwing
  (Development|PrintString "activated")
  (for _array_element (Collision|GetOverlappingActors (Utilities|Select :Index (Variables|Default|GetLastMovement) :NewEnumerator0 (Variables|Default|GetattackHitBoxUp) :NewEnumerator1 (Variables|Default|GetattackHitBoxDown) :NewEnumerator2 (Variables|Default|GetattackHitBoxLeft) :NewEnumerator3 (Variables|Default|GetattackHitBoxRight)) 0 :!class /Script/Engine.PrimitiveComponent)
    (CallFunction|DamageEnemy _array_element)))

(fn EndSwing
  (Components|Activation|SetActive (Utilities|Select :Index (Variables|Default|GetLastMovement) :NewEnumerator0 (Variables|Default|GetattackHitBoxUp) :NewEnumerator1 (Variables|Default|GetattackHitBoxDown) :NewEnumerator2 (Variables|Default|GetattackHitBoxLeft) :NewEnumerator3 (Variables|Default|GetattackHitBoxRight)) false false)
  (Variables|Default|SetBossHit false))