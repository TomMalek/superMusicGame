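; A projectile spell cast by the player that kills enemies and burns wood blocks.
; On spawn it reads the instigating Player's last movement direction and adds a projectile movement component for that direction.
; An overlap cast chain destroys zombies, burns wood blocks and kills charge enemies only while Idle or Tired.
; The spell destroys itself on charge enemies and outer walls, but not on zombies or wood blocks.
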(event EventBeginPlay
  (bind _asplayer (Utilities|Casting|CastToPlayer (Game|GetInstigator)))
  (Variables|Default|SetMy%20Character _asplayer)
  (switch Utilities|FlowControl|Switch|SwitchonMovement (Variables|/Game/blueprints/Player.Player_C|GetLastMovement (Variables|Default|GetMy%20Character))
    (:NewEnumerator0
      (AddComponent|AddProjectileMovementComponent))
    (:NewEnumerator1
      (AddComponent|AddProjectileMovementComponent))
    (:NewEnumerator2
      (AddComponent|AddProjectileMovementComponent))
    (:NewEnumerator3
      (AddComponent|AddProjectileMovementComponent))))

(event Collision|EventActorBeginOverlap
  (params (OtherActor :type Actor%20Object%20Reference))
  (bind _aszombie (Utilities|Casting|CastTozombie OtherActor)
    (:then
      (Actor|DestroyActor OtherActor))
    (:CastFailed
      (bind _aswood_block (Utilities|Casting|CastTowoodBlock OtherActor)
        (:then
          (Default|Burn _aswood_block))
        (:CastFailed
          (bind _ascharge_enemy (Utilities|Casting|CastTochargeEnemy OtherActor)
            (:then
              (switch Utilities|FlowControl|Switch|SwitchonChargeEnum (Variables|/Game/blueprints/chargeEnemy.chargeEnemy_C|GetchargeEnum _ascharge_enemy)
                (:NewEnumerator0
                  (Actor|DestroyActor _ascharge_enemy :!label _label))
                (:NewEnumerator1
                  _)
                (:NewEnumerator2
                  (goto _label)))
              (Actor|DestroyActor))
            (:CastFailed
              (Utilities|Casting|CastToouterWalls OtherActor)
              (Actor|DestroyActor))))))))

(event EventTick
  (params (DeltaSeconds :type Float%20%28single-precision%29)))

(fn ConstructionScript
  (|CallParentFunction))