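; Zombie enemy with a flipbook sprite that chases the first player's pawn and damages it on contact.
; Tick feeds half-strength X and Y movement input toward the player, with a Delay throttling hit checks to about every 0.3 seconds.
; Each check applies Damage through LoseHP to Players overlapping the HitBox.
; Directional attack, walk and idle animation logic sits disconnected, leaving SetAnimation empty.
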(event Custom|testplayerHit
  (for _array_element (Collision|GetOverlappingActors (Variables|Default|GethitBox) "/Game/blueprints/Player.Player_C" :!class /Script/Engine.PrimitiveComponent)
    (bind _asplayer (Utilities|Casting|CastToPlayer _array_element))
    (Default|LoseHP _asplayer (Variables|Default|Getdamage))
    (Development|PrintString "did the dps")))

(event EventBeginPlay)

(event Collision|EventActorBeginOverlap
  (params (OtherActor :type Actor%20Object%20Reference)))

(event EventTick
  (params (DeltaSeconds :type Float%20%28single-precision%29))
  (bind _returnvalue (Transformation|GetActorLocation))
  (bind _returnvalue_2 (Game|Player|GetPlayerPawn 0))
  (bind _returnvalue_3 (Transformation|GetActorLocation _returnvalue_2))
  (bind (_x _y) (Math|Vector|BreakVector _returnvalue))
  (bind (_x_2 _y_2) (Math|Vector|BreakVector _returnvalue_3))
  (Pawn|Input|AddMovementInput "1.000000,0.000000,0.000000" (select (> _x _x_2) -0.5 0.5) false)
  (Pawn|Input|AddMovementInput "0.000000,1.000000, 0" (select (> _y _y_2) -0.5 0.5) false)
  (Utilities|FlowControl|Delay 0.3)
  (CallFunction|TestplayerHit))

(fn ConstructionScript)

(fn SetAnimation)