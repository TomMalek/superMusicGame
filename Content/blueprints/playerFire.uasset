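; Player-fired fire projectile that burns wood blocks, damages the boss and kills charge enemies caught in their Tired state.
; On spawn it reads the instigating player's last movement direction and adds a projectile movement component for it.
; Each tick it polls sphere overlaps after a brief spawn delay, casting each actor to pick the response.
; It destroys itself on enemies, the boss or outer walls, but not on wood blocks.
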(event EventBeginPlay
  (bind _asplayer (Utilities|Casting|CastToPlayer (Game|GetInstigator)))
  (Variables|Default|SetMy%20Character _asplayer)
  (switch Utilities|FlowControl|Switch|SwitchonMovement (Variables|/Game/blueprints/Player.Player_C|GetLastMovement (Variables|Default|GetMy%20Character))
    (:NewEnumerator0
      (AddComponent|AddProjectileMovementComponent))
    (:NewEnumerator1
      (AddComponent|AddProjectileMovementComponent))
    (:NewEnumerator2
      (AddComponent|AddProjectileMovementComponent))
    (:NewEnumerator3
      (AddComponent|AddProjectileMovementComponent))))

(event EventTick
  (params (DeltaSeconds :type Float%20%28single-precision%29))
  (for _array_element (Collision|GetOverlappingActors (Variables|Default|GetSphere) 0 :!class /Script/Engine.PrimitiveComponent)
    (if (> (Actor|GetGameTimeSinceCreation) 0.05)
      (bind _aswood_block (Utilities|Casting|CastTowoodBlock _array_element)
        (:then
          (Default|Burn _aswood_block))
        (:CastFailed
          (bind _ascharge_enemy (Utilities|Casting|CastTochargeEnemy _array_element)
            (:then
              (switch Utilities|FlowControl|Switch|SwitchonChargeEnum (Variables|/Game/blueprints/chargeEnemy.chargeEnemy_C|GetchargeEnum _ascharge_enemy)
                (:NewEnumerator0
                  _)
                (:NewEnumerator1
                  _)
                (:NewEnumerator2
                  (Default|Die _ascharge_enemy)))
              (Actor|DestroyActor))
            (:CastFailed
              (Utilities|Casting|CastToouterWalls _array_element
                (:then
                  (Actor|DestroyActor :!label _label))
                (:CastFailed
                  (bind _asboss (Utilities|Casting|CastToboss _array_element)
                    (:then
                      (Default|BossLoseHP _asboss (Variables|Default|GetfireDamage))
                      (goto _label))
                    (:CastFailed
                      (Utilities|Casting|CastTofireballEnemy _array_element)
                      (Actor|DestroyActor))))))))))))

(fn ConstructionScript
  (|CallParentFunction))