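; Enemy fireball projectile that damages the Player on overlap through LoseHP and prints a debug message.
; On BeginPlay it reads the instigating fireballEnemy's direction type, either following its fixed Up/Down/Left/Right setting or picking one of those four at random.
; It then adds the matching projectile movement component at runtime and takes its lifespan from that enemy's self-destruct timer.
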(event EventBeginPlay
  ;[1 1 1] shoots in wasd directions, can change to shoot in a fixed direction if desired
  (bind _asfireball_enemy (Utilities|Casting|CastTofireballEnemy (Game|GetInstigator)))
  (switch Utilities|FlowControl|Switch|SwitchonfireballDirectionType (Variables|/Game/blueprints/fireballEnemy.fireballEnemy_C|GetdirectionType _asfireball_enemy)
    (:NewEnumerator0
      (switch Utilities|FlowControl|Switch|SwitchonfixedFireballDirection (Variables|/Game/blueprints/fireballEnemy.fireballEnemy_C|Getdirection _asfireball_enemy)
        (:NewEnumerator0
          (AddComponent|AddProjectileMovementComponent :!label _label))
        (:NewEnumerator1
          (AddComponent|AddProjectileMovementComponent :!label _label_2))
        (:NewEnumerator2
          (AddComponent|AddProjectileMovementComponent :!label _label_3))
        (:NewEnumerator3
          (AddComponent|AddProjectileMovementComponent :!label _label_4))))
    (:NewEnumerator1
      (switch int (Utilities|Select :Index (Math|Random|RandomIntegerinRange 0 3) :Option%200 0 :Option%201 1 :Option%202 2 :Option%203 3)
        (:0
          (goto _label))
        (:1
          (goto _label_2))
        (:2
          (goto _label_3))
        (:3
          (goto _label_4)))))
  (bind _asfireball_enemy_2 (Utilities|Casting|CastTofireballEnemy (Game|GetInstigator)))
  (Actor|SetLifeSpan (Variables|/Game/blueprints/fireballEnemy.fireballEnemy_C|GetselfDestructTimer _asfireball_enemy_2)))

(event EventTick
  (params (DeltaSeconds :type Float%20%28single-precision%29)))

(event Collision|EventActorBeginOverlap
  (params (OtherActor :type Actor%20Object%20Reference))
  ;[1 1 1] Enemy version to make the player take damage
  (bind _asplayer (Utilities|Casting|CastToPlayer OtherActor))
  (Default|LoseHP _asplayer (Variables|Default|Getdamage))
  (Development|PrintString "get fireballed kiddo"))

(fn ConstructionScript
  (|CallParentFunction))