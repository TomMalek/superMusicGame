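; Enemy character with a flipbook sprite that chases the player and damages them on contact.
; Each tick it compares its X and Y position to the player pawn's and adds half-scale movement input toward it on each axis.
; HitBox overlap with a Player calls LoseHP with Damage and prints debug text.
; SetAnimation is empty: its directional attack, walk and stand flipbook selection is disconnected, as are the MoveEnemyH/V assignments.
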(event OnComponentBeginOverlap(hitBox)
  (params (OverlappedComponent :type Primitive%20Component%20Object%20Reference) (OtherActor :type Actor%20Object%20Reference) (OtherComp :type Primitive%20Component%20Object%20Reference) (OtherBodyIndex :type Integer) (bFromSweep :type Boolean) (SweepResult :type Hit%20Result%20Structure%20%28by%20ref%29))
  (if (== (Utilities|GetClass OtherActor) "/Game/blueprints/Player.Player_C")
    (bind _asplayer (Utilities|Casting|CastToPlayer (Game|Player|GetPlayerPawn 0))
      (:then
        (Default|LoseHP _asplayer (Variables|Default|Getdamage))
        (Development|PrintString "Hello"))
      (:CastFailed
        (Development|PrintString "shits fucked")))))

(event EventBeginPlay)

(event Collision|EventActorBeginOverlap
  (params (OtherActor :type Actor%20Object%20Reference)))

(event EventTick
  (params (DeltaSeconds :type Float%20%28single-precision%29))
  (bind _returnvalue (Transformation|GetActorLocation))
  (bind _returnvalue_2 (Game|Player|GetPlayerPawn 0))
  (bind _returnvalue_3 (Transformation|GetActorLocation _returnvalue_2))
  (bind (_x _y) (Math|Vector|BreakVector _returnvalue))
  (bind (_x_2 _y_2) (Math|Vector|BreakVector _returnvalue_3))
  (Pawn|Input|AddMovementInput "1.000000,0.000000,0.000000" (select (> _x _x_2) -0.5 0.5) false)
  (Pawn|Input|AddMovementInput "0.000000,1.000000, 0" (select (> _y _y_2) -0.5 0.5) false))

(fn ConstructionScript)

(fn SetAnimation)