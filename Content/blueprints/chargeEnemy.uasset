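; Charger enemy, a flipbook-animated bat that wanders, charges at one of two players and then tires.
; Tick sets the animation and movement for the current state, while Delay nodes on Tick act as state timers before UpdateState advances Idle, Charge and Tired.
; Idle jitters randomly; Charge steers by X/Y sign toward a randomly picked player.
; Capsule hits while Idle or Charging apply delayed damage, whose amount UpdateState changes.
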(event OnComponentHit(CapsuleComponent)
  (params (HitComponent :type Primitive%20Component%20Object%20Reference) (OtherActor :type Actor%20Object%20Reference) (OtherComp :type Primitive%20Component%20Object%20Reference) (NormalImpulse :type Vector :default "0, 0, 0") (Hit :type Hit%20Result%20Structure%20%28by%20ref%29))
  ;[1 1 1] damages player on contact when not tired
  (if (== (Utilities|GetClass OtherActor) "/Game/blueprints/Player.Player_C")
    (switch Utilities|FlowControl|Switch|SwitchonChargeEnum (Variables|Default|GetchargeEnum)
      (:NewEnumerator0
        _)
      (:NewEnumerator1
        _))
    (bind _asplayer (Utilities|Casting|CastToPlayer OtherActor)
      (:then
        (Utilities|FlowControl|Delay 0.25)
        (Default|LoseHP _asplayer (Variables|Default|Getdamage))
        (Development|PrintString "dealt dmg from charger"))
      (:CastFailed
        (Development|PrintString "busted")))))

(event Custom|actBasedOnState
  ;[1 1 1] determines actions based on state
  (switch Utilities|FlowControl|Switch|SwitchonChargeEnum (Variables|Default|GetchargeEnum)
    (:NewEnumerator0
      (CallFunction|Idle))
    (:NewEnumerator1
      (CallFunction|Charge))))

(event EventBeginPlay
  (Development|PrintString "is alive"))

(event Collision|EventActorBeginOverlap
  (params (OtherActor :type Actor%20Object%20Reference)))

(event EventTick
  (params (DeltaSeconds :type Float%20%28single-precision%29))
  ;[1 1 1] determines state of charge enemy based on timers
  (CallFunction|SetAnimation)
  (CallFunction|ActBasedonState)
  (switch Utilities|FlowControl|Switch|SwitchonChargeEnum (Variables|Default|GetchargeEnum)
    (:NewEnumerator0
      (Utilities|FlowControl|Delay (Math|Conversions|ToFloat(Integer) (Math|Random|RandomIntegerinRange 3 9))))
    (:NewEnumerator1
      (Utilities|FlowControl|Delay 0.9))
    (:NewEnumerator2
      (Utilities|FlowControl|Delay 3.0)))
  (CallFunction|UpdateState))

(fn ConstructionScript)

(fn UpdateState
  (switch Utilities|FlowControl|Switch|SwitchonChargeEnum (Variables|Default|GetchargeEnum)
    (:NewEnumerator0
      (Variables|Default|SettargetPlayer (Math|Random|RandomIntegerinRange 0 1))
      (Variables|Default|SetchargeEnum "NewEnumerator1"))
    (:NewEnumerator1
      (Variables|Default|SetchargeEnum "NewEnumerator2")
      (Variables|Default|Setdamage 5))
    (:NewEnumerator2
      (Variables|Default|SetchargeEnum "NewEnumerator0")
      (Variables|Default|Setdamage 1))))

(fn Charge
  (bind _returnvalue (Transformation|GetActorLocation))
  (bind _targetplayer (Variables|Default|GettargetPlayer))
  (bind _returnvalue_2 (Game|Player|GetPlayerPawn _targetplayer))
  (bind (_x _y) (Math|Vector|BreakVector _returnvalue))
  (bind _returnvalue_3 (Transformation|GetActorLocation _returnvalue_2))
  (bind (_x_2 _y_2) (Math|Vector|BreakVector _returnvalue_3))
  (Pawn|Input|AddMovementInput "1.000000,0.000000,0.000000" (select (> _x _x_2) -1.0 1.0) false)
  (Pawn|Input|AddMovementInput "0.000000,1.000000, 0" (select (> _y _y_2) -1.0 1.0) false))

(fn Idle
  (bind _output_get (Variables|Default|SetrandomDirection (Math|Vector|MakeVector (Math|Conversions|ToFloat(Integer) (Math|Random|RandomIntegerinRange -1 1)) (Math|Conversions|ToFloat(Integer) (Math|Random|RandomIntegerinRange -1 1)) 0.0)))
  (Pawn|Input|AddMovementInput _output_get 0.3 false))

(fn SetAnimation
  (bind _flipbook (Variables|Default|GetflipBook))
  (switch Utilities|FlowControl|Switch|SwitchonChargeEnum (Variables|Default|GetchargeEnum)
    (:NewEnumerator0
      (Sprite|SetFlipbook _flipbook "/Game/FlipBooks/batIdle.batIdle"))
    (:NewEnumerator1
      (Sprite|SetFlipbook _flipbook "/Game/FlipBooks/batCharge.batCharge"))
    (:NewEnumerator2
      (Sprite|SetFlipbook _flipbook "/Game/FlipBooks/batTired.batTired"))))