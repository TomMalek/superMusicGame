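; 2D boss actor that stays shielded while bats are alive and only takes damage once vulnerable.
; Tick swaps the shielded or vulnerable flipbook, toggles the particle effect and, while shielded, uses a Delay to spawn EnemySpell about every 1.5 seconds.
; UpdateVulnerablee sets vulnerability from the game instance's BatsAlive count.
; BossLoseHP subtracts HP when vulnerable and destroys the boss at zero or below.
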(event Custom|batsAlive
  (Utilities|FlowControl|Delay 1.5)
  (if (not (Variables|Default|Getvulnerable))
    (Game|SpawnActorfromClass "/Game/blueprints/enemySpell.enemySpell_C" (Math|Transform|MakeTransform (- (Transformation|GetActorLocation self) "35.000000,17.000000, 0") "0, 0, 0" "0.500000,0.500000,0.500000") "Undefined" 0 self)))

(event EventBeginPlay)

(event Collision|EventActorBeginOverlap
  (params (OtherActor :type Actor%20Object%20Reference)))

(event EventTick
  (params (DeltaSeconds :type Float%20%28single-precision%29))
  (if (Variables|Default|Getvulnerable)
    _
    (else
      (CallFunction|BatsAlive)))
  (CallFunction|SetAnimation)
  (Development|SetHiddeninGame (Variables|Default|GetParticleSystem) (Variables|Default|Getvulnerable) false))

(fn ConstructionScript)

(fn BossLoseHP
  (params (damage :type Integer))
  (if (Variables|Default|Getvulnerable)
    (Variables|Default|SetbossHP (- (Variables|Default|GetbossHP) damage))
    (Math|Integer|CompareInt (Variables|Default|GetbossHP) 0
      (:==
        _)
      (:<
        _))
    (Variables|Default|SetbossIsDead true)
    (Development|PrintString "killed the boss")
    (Actor|DestroyActor)
    (else
      (Development|PrintString "more enemies around"))))

(fn SetAnimation
  (bind _paperflipbook (Variables|Default|GetPaperFlipbook))
  (if (Variables|Default|Getvulnerable)
    (Sprite|SetFlipbook _paperflipbook "/Game/FlipBooks/bossVulnerable2.bossVulnerable2")
    (else
      (Sprite|SetFlipbook _paperflipbook "/Game/FlipBooks/bossShielded2.bossShielded2"))))

(fn UpdateVulnerablee
  (bind _asinstance_blueprint (Utilities|Casting|CastToinstanceBlueprint (Game|GetGameInstance)))
  (Variables|Default|Setvulnerable (== (Variables|/Game/blueprints/instanceBlueprint.instanceBlueprint_C|GetbatsAlive _asinstance_blueprint) 0)))