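; Trigger volume actor that activates the spawn points of a room when the player walks into it.
; On overlap by an actor of the Player class, it runs TriggerSpawners and then destroys itself, so it fires only once.
; TriggerSpawners scans every SpawnPointBlueprint in the level and sets Activated on those whose room number matches its SpawnRoomNumber.
; A direct SpawnObject call is left disconnected.
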(event OnComponentBeginOverlap(CollisionComponent)
  (params (OverlappedComponent :type Primitive%20Component%20Object%20Reference) (OtherActor :type Actor%20Object%20Reference) (OtherComp :type Primitive%20Component%20Object%20Reference) (OtherBodyIndex :type Integer) (bFromSweep :type Boolean) (SweepResult :type Hit%20Result%20Structure%20%28by%20ref%29))
  (if (== (Utilities|GetClass OtherActor) "/Game/blueprints/Player.Player_C")
    (CallFunction|TriggerSpawners)
    (Actor|DestroyActor)))

(event EventBeginPlay)

(event Collision|EventActorBeginOverlap
  (params (OtherActor :type Actor%20Object%20Reference)))

(event EventTick
  (params (DeltaSeconds :type Float%20%28single-precision%29)))

(fn ConstructionScript)

(fn TriggerSpawners
  (bind _outactors (Actor|GetAllActorsOfClass "/Game/blueprints/spawnPointBlueprint.spawnPointBlueprint_C"))
  (for _array_element _outactors
    (bind _asspawn_point_blueprint (Utilities|Casting|CastTospawnPointBlueprint _array_element))
    (if (== (Variables|/Game/blueprints/spawnPointBlueprint.spawnPointBlueprint_C|GetpointRoomNumber _asspawn_point_blueprint) (Variables|Default|GetspawnRoomNumber))
      (Variables|/Game/blueprints/spawnPointBlueprint.spawnPointBlueprint_C|Setactivated _asspawn_point_blueprint true))))