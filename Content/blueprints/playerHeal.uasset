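; Healing projectile actor that restores HP to a Player it touches.
; On BeginPlay it reads the instigating player's last movement direction and adds a projectile movement component for that direction.
; Each tick it polls its sphere for overlapping Players, ignoring them for a brief delay after spawn, then adds a fixed amount of HP capped at MaxHP and destroys itself.
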(event EventBeginPlay
  (bind _asplayer (Utilities|Casting|CastToPlayer (Game|GetInstigator)))
  (Variables|Default|SetMy%20Character _asplayer)
  (switch Utilities|FlowControl|Switch|SwitchonMovement (Variables|/Game/blueprints/Player.Player_C|GetLastMovement (Variables|Default|GetMy%20Character))
    (:NewEnumerator0
      (AddComponent|AddProjectileMovementComponent))
    (:NewEnumerator1
      (AddComponent|AddProjectileMovementComponent))
    (:NewEnumerator2
      (AddComponent|AddProjectileMovementComponent))
    (:NewEnumerator3
      (AddComponent|AddProjectileMovementComponent))))

(event EventTick
  (params (DeltaSeconds :type Float%20%28single-precision%29))
  (for _array_element (Collision|GetOverlappingActors (Variables|Default|GetSphere) "/Game/blueprints/Player.Player_C" :!class /Script/Engine.PrimitiveComponent)
    (if (> (Actor|GetGameTimeSinceCreation) 0.1)
      (bind _asplayer (Utilities|Casting|CastToPlayer _array_element))
      (Math|Integer|CompareInt (+ (Variables|/Game/blueprints/Player.Player_C|GetHP _asplayer) 10) (Variables|/Game/blueprints/Player.Player_C|GetmaxHP _asplayer)
        (:>
          (Variables|/Game/blueprints/Player.Player_C|SetHP _asplayer (Variables|/Game/blueprints/Player.Player_C|GetmaxHP _asplayer)))
        (:==
          (Variables|/Game/blueprints/Player.Player_C|SetHP _asplayer (+ (Variables|/Game/blueprints/Player.Player_C|GetHP _asplayer) 10) :!label _label))
        (:<
          (goto _label)))
      (Actor|DestroyActor))))

(fn ConstructionScript
  (|CallParentFunction))