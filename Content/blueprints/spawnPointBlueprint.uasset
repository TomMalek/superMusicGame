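; Spawn point actor that spawns AI pawns of a chosen class at its own location and rotation.
; Setting Activated makes Tick spawn one pawn immediately, clear the flag and start spawning mode.
; If EndlessSpawner is set, Tick then switches the class to ChargeEnemy and repeatedly spawns through a Delay, resetting SpawnDelay after each spawn.
; The BeginPlay delay leads to nothing.
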(event EventBeginPlay
  (Utilities|FlowControl|Delay 11.0))

(event Collision|EventActorBeginOverlap
  (params (OtherActor :type Actor%20Object%20Reference)))

(event EventTick
  (params (DeltaSeconds :type Float%20%28single-precision%29))
  (if (Variables|Default|Getactivated)
    (CallFunction|SpawnObject)
    (Variables|Default|SetstartSpawning true)
    (Variables|Default|Setactivated false)
    (elif (Variables|Default|GetstartSpawning)
      (if (Variables|Default|GetendlessSpawner)
        (Variables|Default|SetspawnClass "/Game/blueprints/chargeEnemy.chargeEnemy_C")
        (Utilities|FlowControl|Delay (Variables|Default|GetspawnDelay))
        (CallFunction|SpawnObject)
        (Variables|Default|SetspawnDelay 2e+01)))))

(fn ConstructionScript)

(fn SpawnObject
  (bind _aspawn (Utilities|Casting|CastToPawnClass (Variables|Default|GetspawnClass)))
  (AI|SpawnAIFromClass _aspawn 0 (Transformation|GetActorLocation) (Transformation|GetActorRotation) true))